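; Player controller for what appears to be a guessing game, creating the HUD and relaying guesses and messages.
; On BeginPlay it creates WBP_GameHUD and adds it to the viewport, only for the local controller.
; Pressing G calls SendGuess with an empty string.
; OnMessageReceived stores the incoming text in LastMessage and prints it on screen.
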(event `Key|G`
  (params (Key :type "Key Structure"))
  (:`Pressed`
    (`self.SendGuess` "")))

(event `self.OnMessageReceived`
  (params (Message :type String))
  (bind _output_get (set `self.LastMessage` Message))
  (`KismetSystemLibrary.PrintString` _output_get true true (struct :`G` 0.66 :`B` 1.0 :`A` 1.0) 15.0))

(event `self.ReceiveBeginPlay`
  (if (`self.IsLocalController`)
    (bind _returnvalue (`|CreateWidget` "/Game/Blueprints/WBP_GameHUD.WBP_GameHUD_C" self))
    (bind _output_get (set `self.GameHUD` _returnvalue))
    (`UserWidget.AddToViewport` _output_get 0)))

(fn `UserConstructionScript`)